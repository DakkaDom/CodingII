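; Fireball projectile that destroys itself on hit and deals radial damage within its configured radius.
; The Hit event runs a debug-drawn sphere trace on the Camera channel from the impact point to the actor's location.
; A successful trace applies radial damage at the trace start, credited to the first player controller.
; An unconnected older branch with per-enemy casts and damage reporting never runs, and the component hit event is empty.
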(event `self.ReceiveHit`
  (params (MyComp :type "PrimitiveComponent Object Reference") (Other :type "Actor Object Reference") (OtherComp :type "PrimitiveComponent Object Reference") (bSelfMoved :type Boolean) (HitLocation :type "Vector Structure") (HitNormal :type "Vector Structure") (NormalImpulse :type "Vector Structure") (Hit :type "HitResult Structure (by ref)"))
  ;[0.1243 0 1] When the fireball hits an object, deal damage in a set radius
  (`self.K2_DestroyActor`)
  (bind (_outhit _returnvalue) (`KismetSystemLibrary.SphereTraceSingle` :`Start` HitLocation :`End` (`self.K2_GetActorLocation`) :`Radius` (`self.FireballRadius`) :`TraceChannel` "TraceTypeQuery2" :`bTraceComplex` true :`DrawDebugType` "ForDuration"))
  (if _returnvalue
    (`GameplayStatics.ApplyRadialDamage` :`BaseDamage` (`self.FireballDamage`) :`Origin` (`.TraceStart` (`GameplayStatics.BreakHitResult` _outhit)) :`DamageRadius` (`self.FireballRadius`) :`DamageCauser` self :`InstigatedByController` (`GameplayStatics.GetPlayerController` 0))))

(event `self.Fireball.OnComponentHit`
  (params (HitComponent :type "PrimitiveComponent Object Reference") (OtherActor :type "Actor Object Reference") (OtherComp :type "PrimitiveComponent Object Reference") (NormalImpulse :type "Vector Structure") (Hit :type "HitResult Structure (by ref)"))
  ;[0.5052 0.00016 0.007773] THE BIT WHERE I WILDLY OVERCOMPLICATED IT
)

(fn `UserConstructionScript`)