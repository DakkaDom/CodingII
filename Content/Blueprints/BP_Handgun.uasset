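; BP_Handgun is a pickup weapon with primary and secondary fire that can be picked up and dropped.
; Pickup attaches it to the given skeletal mesh's BPI_ItemSocket and disables Box collision.
; Primary and secondary fire spawn BP_Projectile or BP_Fan at the Box transform and push them forward with a large force.
; Dropping detaches the gun, spawns a fresh BP_Handgun in its place and destroys the original.
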(event `PickupItem`
  (params (SkeletalMesh :type "SkeletalMeshComponent Object Reference"))
  ; Picks up the gun
  (`KismetSystemLibrary.PrintText` "This gun is getting picked up!")
  (`self.K2_AttachToComponent` SkeletalMesh "BPI_ItemSocket" "SnapToTarget" "KeepRelative" "KeepRelative")
  (`PrimitiveComponent.SetCollisionEnabled` (`self.Box`) "NoCollision"))

(event `/Game/Blueprints/BPI_Item.UsePrimary`
  ; Shoots a projectile when LMB is pressed
  (`KismetSystemLibrary.PrintText` "Activating primary action")
  (bind _returnvalue (`|SpawnActorFromClass` "/Game/Blueprints/BP_Projectile.BP_Projectile_C" (`SceneComponent.K2_GetComponentToWorld` (`self.Box`)) "Undefined" "MultiplyWithRoot" null null))
  (`PrimitiveComponent.AddForce` (`/Game/Blueprints/BP_Projectile.Sphere` _returnvalue) (* (`SceneComponent.GetForwardVector` (`self.Box`)) 500000.0) "None" true))

(event `/Game/Blueprints/BPI_Item.UseSecondary`
  ; Shoot a second projectile when RMB is pressed
  (`KismetSystemLibrary.PrintText` "Activating secondary action")
  (bind _returnvalue (`|SpawnActorFromClass` "/Game/Blueprints/BP_Fan.BP_Fan_C" (`SceneComponent.K2_GetComponentToWorld` (`self.Box`)) "Undefined" "MultiplyWithRoot" null null))
  (`PrimitiveComponent.AddForce` (`/Game/Blueprints/BP_Fan.FanBlade` _returnvalue) (* (`SceneComponent.GetForwardVector` (`self.Box`)) 500000.0) "None" false))

(event `/Game/Blueprints/BPI_Item.Drop`
  ; Drops gun
  (`KismetSystemLibrary.PrintText` "Dropping item")
  (`self.K2_DetachFromActor` "KeepWorld")
  (`|SpawnActorFromClass` "BP_Handgun_C" (`self.GetTransform`) "Undefined" "MultiplyWithRoot" null null)
  (`self.K2_DestroyActor`))

(fn `Pickup`
  (params (SkeletalMesh :type "SkeletalMeshComponent Object Reference"))
  (returns (Item :type String))
  (`KismetSystemLibrary.PrintString` "Item Picked Up")
  (return (`self.Item`)))

(fn `UserConstructionScript`)