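; Game mode that saves and loads player stats and per-level collected-coin state through two SaveGame objects.
; On BeginPlay it loads each save or creates a new one, copying Stamina, Health and Mana onto the third-person character.
; Level state uses the level name as its slot, and loading replays CollectThyself on each valid saved coin.
; Save events write the held objects as they are, without gathering current values.
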(event `self.ReceiveBeginPlay`
  (`KismetSystemLibrary.PrintString` "Loading the SaveLoad Game Mode" true true (struct :`R` 1.0 :`B` 0.689684 :`A` 1.0) 10.0)
  (`self.Load Player Stats`)
  (`self.Load Level State`))

(event `Load Player Stats`
  (bind _returnvalue (`GameplayStatics.DoesSaveGameExist` (`self.PlayerStatsSave`)))
  (if _returnvalue
    (bind _returnvalue_2 (`GameplayStatics.LoadGameFromSlot` (`self.PlayerStatsSave`)))
    (`/Engine/EditorBlueprintResources/StandardMacros.IsValid` _returnvalue_2
      (:`Is Valid`
        (bind _assg_player_stats (cast `/Game/Blueprints/Saving_and_Loading/SG_PlayerStats` _returnvalue_2)
          (:`then`
            (set `self.SG_PlayerStats` _assg_player_stats)
            (`|ExecutionSequence`
              (:`then_0`
                (bind _asbp_third_person_character (cast `/Game/ThirdPerson/Blueprints/BP_ThirdPersonCharacter` (`GameplayStatics.GetPlayerCharacter` 0))
                  (:`then`
                    (set `/Game/ThirdPerson/Blueprints/BP_ThirdPersonCharacter.Stamina` (`/Game/Blueprints/Saving_and_Loading/SG_PlayerStats.Stamina` (`self.SG_PlayerStats`)) _asbp_third_person_character)
                    (`KismetSystemLibrary.PrintString` "Player Stamina has been loaded." true true (struct :`G` 0.421875 :`B` 0.006836 :`A` 1.0)))
                  (:`CastFailed`
                    (`KismetSystemLibrary.PrintString` "STAMINA NOT LOADED" true true (struct :`R` 0.505208 :`G` 0.00016 :`B` 0.007773 :`A` 1.0) 10.0))))
              (:`then_1`
                (bind _asbp_third_person_character_2 (cast `/Game/ThirdPerson/Blueprints/BP_ThirdPersonCharacter` (`GameplayStatics.GetPlayerCharacter` 0))
                  (:`then`
                    (set `/Game/ThirdPerson/Blueprints/BP_ThirdPersonCharacter.Health` (`/Game/Blueprints/Saving_and_Loading/SG_PlayerStats.Health` (`self.SG_PlayerStats`)) _asbp_third_person_character_2)
                    (`KismetSystemLibrary.PrintString` "Player Health has been loaded." true true (struct :`G` 0.421875 :`B` 0.006836 :`A` 1.0)))
                  (:`CastFailed`
                    (`KismetSystemLibrary.PrintString` "HEALTH NOT LOADED" true true (struct :`R` 0.505208 :`G` 0.00016 :`B` 0.007773 :`A` 1.0) 10.0))))
              (:`then_2`
                (bind _asbp_third_person_character_3 (cast `/Game/ThirdPerson/Blueprints/BP_ThirdPersonCharacter` (`GameplayStatics.GetPlayerCharacter` 0))
                  (:`then`
                    (set `/Game/ThirdPerson/Blueprints/BP_ThirdPersonCharacter.Mana` (`/Game/Blueprints/Saving_and_Loading/SG_PlayerStats.Mana` (`self.SG_PlayerStats`)) _asbp_third_person_character_3)
                    (`KismetSystemLibrary.PrintString` "Player Mana has been loaded." true true (struct :`G` 0.421875 :`B` 0.006836 :`A` 1.0)))
                  (:`CastFailed`
                    (`KismetSystemLibrary.PrintString` "MANA NOT LOADED" true true (struct :`R` 0.505208 :`G` 0.00016 :`B` 0.007773 :`A` 1.0) 10.0))))))
          (:`CastFailed`
            (`KismetSystemLibrary.PrintText` "LOAD STATS FAILED" true true (struct :`R` 0.505208 :`G` 0.00016 :`B` 0.007773 :`A` 1.0) 20.0))))
      (:`Is Not Valid`
        (`KismetSystemLibrary.PrintText` "SG_PlayerStats is not valid Load Game" true true (struct :`R` 1.0 :`G` 0.408347 :`A` 1.0) 10.0)))
    (else
      (bind _returnvalue_3 (`GameplayStatics.CreateSaveGameObject` "/Game/Blueprints/Saving_and_Loading/SG_PlayerStats.SG_PlayerStats_C"))
      (set `self.SG_PlayerStats` _returnvalue_3))))

(event `Save Player Stats`
  (bind _returnvalue (`GameplayStatics.SaveGameToSlot` (`self.SG_PlayerStats`) (`self.PlayerStatsSave`)))
  (if _returnvalue
    (`KismetSystemLibrary.PrintText` "Player Stats Written to Save Game File" true true (struct :`R` 0.00077 :`G` 0.401042 :`B` 0.02197 :`A` 1.0))
    (else
      (`KismetSystemLibrary.PrintText` "Player Stats Could Not be Written to Save Game File" true true (struct :`R` 0.505208 :`G` 0.00016 :`B` 0.007773 :`A` 1.0)))))

(event `Load Level State`
  (bind _returnvalue (`GameplayStatics.GetCurrentLevelName` true))
  (bind _returnvalue_2 (`GameplayStatics.DoesSaveGameExist` _returnvalue))
  (if _returnvalue_2
    (bind _returnvalue_3 (`GameplayStatics.LoadGameFromSlot` _returnvalue))
    (bind _assg_level_state (cast `/Game/Blueprints/Saving_and_Loading/SG_LevelState` _returnvalue_3)
      (:`then`
        (bind _output_get (set `self.SG_LevelState` _assg_level_state))
        (for _array_element (`/Game/Blueprints/Saving_and_Loading/SG_LevelState.CollectedCoins` _output_get)
          (`/Engine/EditorBlueprintResources/StandardMacros.IsValid` _array_element
            (:`Is Valid`
              (`/Game/Blueprints/BP_Coin.CollectThyself` _array_element))))
        (`KismetSystemLibrary.PrintText` "Coin States Have Been Loaded" true true (struct :`R` 0.986829 :`G` 0.001713 :`B` 1.0 :`A` 1.0) 4.0))
      (:`CastFailed`
        (`KismetSystemLibrary.PrintText` "LOAD LEVEL STATE FAILED" true true (struct :`R` 0.741319 :`B` 0.020888 :`A` 1.0) 20.0)))
    (else
      (bind _returnvalue_4 (`GameplayStatics.CreateSaveGameObject` "/Game/Blueprints/Saving_and_Loading/SG_LevelState.SG_LevelState_C"))
      (set `self.SG_LevelState` _returnvalue_4))))

(event `Save Level State`
  (bind _returnvalue (`GameplayStatics.GetCurrentLevelName` true))
  (bind _returnvalue_2 (`GameplayStatics.SaveGameToSlot` (`self.SG_LevelState`) _returnvalue))
  (if _returnvalue_2
    (`KismetSystemLibrary.PrintText` "Level State Written to Save Game File" true true (struct :`R` 1.0 :`B` 0.689684 :`A` 1.0))
    (else
      (`KismetSystemLibrary.PrintText` "Level State Could Not be Written to Save Game File" true true (struct :`R` 0.505208 :`G` 0.00016 :`B` 0.007773 :`A` 1.0)))))

(fn `UserConstructionScript`)