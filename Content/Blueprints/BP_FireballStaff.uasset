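; BP_FireballStaff is a pickup weapon that casts fireballs using the player's mana.
; Pickup snaps it to a socket on the supplied skeletal mesh and disables box collision; Drop spawns a fresh staff and destroys this one.
; Primary use spawns BP_Fireball with sound at ProjectileSpawnPos, deducts mana from player 0's character, then clears CanCast if mana is too low.
; CanCast is only re-evaluated after a successful cast.
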(event `PickupItem`
  (params (SkeletalMesh :type "SkeletalMeshComponent Object Reference"))
  ; Picks up the staff and places it in the player's hand
  (if true
    (`KismetSystemLibrary.PrintString` "Staff is being picked up!")
    (`self.K2_AttachToComponent` SkeletalMesh "BPI_ItemSocket" "SnapToTarget" "SnapToTarget" "KeepRelative")
    (`PrimitiveComponent.SetCollisionEnabled` (`self.Box`) "NoCollision")
    (else
      (`KismetSystemLibrary.PrintString` "Could not pick up staff!"))))

(event `/Game/Blueprints/BPI_Item.UsePrimary`
  (bind (_returnvalue_location _returnvalue_rotation) (`KismetMathLibrary.BreakTransform` (`SceneComponent.K2_GetComponentToWorld` (`self.ProjectileSpawnPos`))))
  ; Shoots a fireball for primary action
  (if (`self.CanCast`)
    (`KismetSystemLibrary.PrintString` "FIREBALL" true true (struct :`R` 1.0 :`G` 0.35757 :`A` 1.0))
    (`|SpawnActorFromClass` "/Game/Blueprints/BP_Fireball.BP_Fireball_C" (`KismetMathLibrary.MakeTransform` _returnvalue_location _returnvalue_rotation (0.75 0.75 0.75)) "AlwaysSpawn" "MultiplyWithRoot" null null)
    (`GameplayStatics.PlaySoundAtLocation` "/Game/Audio/SC_Fireball.SC_Fireball" _returnvalue_location (struct) 1.0 1.0 0.0 null null null null)
    (bind _asbp_third_person_character (cast `/Game/ThirdPerson/Blueprints/BP_ThirdPersonCharacter` (`GameplayStatics.GetPlayerCharacter` 0)))
    (`/Game/ThirdPerson/Blueprints/BP_ThirdPersonCharacter.ChangeMana` _asbp_third_person_character -0.2)
    (if (<= (`/Game/ThirdPerson/Blueprints/BP_ThirdPersonCharacter.Mana` _asbp_third_person_character) 0.19)
      (set `self.CanCast` false)
      (else
        (set `self.CanCast` true)))
    (else
      (`KismetSystemLibrary.PrintString` "Player is out of mana!"))))

(event `/Game/Blueprints/BPI_Item.Drop`
  ; Drops the staff when Event Drop is called
  (`KismetSystemLibrary.PrintString` "Dropping item")
  (`|SpawnActorFromClass` "BP_FireballStaff_C" (`self.GetTransform`) "AdjustIfPossibleButAlwaysSpawn" "MultiplyWithRoot" null null)
  (`self.K2_DestroyActor`))

(fn `Pickup`
  (params (SkeletalMesh :type "SkeletalMeshComponent Object Reference"))
  (returns (Item :type String))
  (return ""))

(fn `UserConstructionScript`)