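; Spawn manager actor that populates the level with AI enemies when play begins.
; It finds every BP_EnemySpawnPoint, prints the count, and gives each a random coin flip to spawn a BP_AiMoveTo at its transform, owned by that point.
; Each spawned AI gets its name text set to a random entry from the Names array on BP_ThirdPersonGameMode.
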(event `self.ReceiveBeginPlay`
  ;[0.6771 0 0.03844 0.5] Spawns AI entities
  (bind _outactors (`GameplayStatics.GetAllActorsOfClass` "/Game/Blueprints/BP_EnemySpawnPoint.BP_EnemySpawnPoint_C"))
  (`KismetSystemLibrary.PrintText` (`|FormatText` "There are {count} spawn points in this level" (`KismetArrayLibrary.Array_Length` _outactors)))
  (for _array_element _outactors
    (if (`KismetMathLibrary.RandomBool`)
      (bind _returnvalue (`|SpawnActorFromClass` "/Game/AI_Blueprints/BP_AiMoveTo.BP_AiMoveTo_C" (`self.GetTransform` _array_element) "Undefined" "MultiplyWithRoot" _array_element null))
      ;[0.8594 0.001828 0.7684 0.5] Randomizes entity names
      (bind _asbp_third_person_game_mode (cast `/Game/ThirdPerson/Blueprints/BP_ThirdPersonGameMode` (`GameplayStatics.GetGameMode`)))
      (bind _names (`/Game/ThirdPerson/Blueprints/BP_ThirdPersonGameMode.Names` _asbp_third_person_game_mode))
      (`TextRenderComponent.K2_SetText` (`/Game/AI_Blueprints/BP_AiMoveTo.AI_NameText` _returnvalue) (`|GetArrayItem` _names (`KismetMathLibrary.RandomInteger` (`KismetArrayLibrary.Array_Length` _names)))))))

(fn `UserConstructionScript`)