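; BP_ManaRestore is a mana potion item the player can pick up, use and drop.
; Pickup snaps it to the BPI_ItemSocket socket on the given skeletal mesh and disables its box collision.
; Primary use adds mana to player 0's third-person character, changes the sphere to glass and marks it empty, without blocking repeat use.
; Drop replaces the actor with a fresh full or empty potion at its location.
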(event `PickupItem`
  (params (`Skeletal Mesh` :type "SkeletalMeshComponent Object Reference"))
  ; Picks up the health potion
  (if true
    (`KismetSystemLibrary.PrintString` "Picking up mana potion")
    (`self.K2_AttachToComponent` `Skeletal Mesh` "BPI_ItemSocket" "SnapToTarget" "SnapToTarget" "KeepRelative")
    (`PrimitiveComponent.SetCollisionEnabled` (`self.Box`) "NoCollision")
    (else
      (`KismetSystemLibrary.PrintString` "Could not pick up mana potion"))))

(event `self.UsePrimary`
  ; Restores player mana on use
  (bind _asbp_third_person_character (cast `/Game/ThirdPerson/Blueprints/BP_ThirdPersonCharacter` (`GameplayStatics.GetPlayerCharacter` 0)))
  (`/Game/ThirdPerson/Blueprints/BP_ThirdPersonCharacter.ChangeMana` _asbp_third_person_character 0.4)
  (`PrimitiveComponent.SetMaterial` (`self.Sphere`) 0 "/DatasmithContent/Materials/FBXImporter/VRED/Glass.Glass")
  (set `self.Empty` true))

(event `self.Drop`
  (bind (_returnvalue_location _returnvalue_rotation _returnvalue_scale) (`KismetMathLibrary.BreakTransform` (`self.GetTransform`)))
  (bind (_returnvalue_location_2 _returnvalue_rotation_2 _returnvalue_scale_2) (`KismetMathLibrary.BreakTransform` (`self.GetTransform`)))
  ; Drops an empty potion if empty, drops a full potion if full
  (`KismetSystemLibrary.PrintString` "Dropping item")
  (if (`self.Empty`)
    (`|SpawnActorFromClass` "/Game/Blueprints/BP_EmptyPotion.BP_EmptyPotion_C" (`KismetMathLibrary.MakeTransform` _returnvalue_location (struct) _returnvalue_scale) "Undefined" "MultiplyWithRoot" null null)
    (`self.K2_DestroyActor`)
    (else
      (`|SpawnActorFromClass` "BP_ManaRestore_C" (`KismetMathLibrary.MakeTransform` _returnvalue_location_2 (struct) _returnvalue_scale_2) "Undefined" "MultiplyWithRoot" null null)
      (`self.K2_DestroyActor`))))

(fn `Pickup`
  (params (SkeletalMesh :type "SkeletalMeshComponent Object Reference"))
  (returns (Item :type String))
  (return ""))

(fn `UserConstructionScript`)