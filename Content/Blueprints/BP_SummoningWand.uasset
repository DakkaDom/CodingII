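; BP_SummoningWand is a holdable item actor that can be picked up, used and dropped.
; Pickup snaps it to a socket on the given skeletal mesh and disables its box collision.
; Primary use spawns a BP_AiMoveTo at the wand's transform, while secondary use toggles the cylinder between emissive pink and base materials.
; Drop detaches it, spawns a fresh wand in place and destroys itself.
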(event `/Game/Blueprints/BPI_Item.Pickup`
  (params (SkeletalMesh :type "SkeletalMeshComponent Object Reference"))
  ; Picks up the wand
  (`KismetSystemLibrary.PrintText` "This wand is getting picked up!")
  (`self.K2_AttachToComponent` SkeletalMesh "BPI_ItemSocket" "SnapToTarget" "SnapToTarget" "KeepRelative")
  (`PrimitiveComponent.SetCollisionEnabled` (`self.Box`) "NoCollision"))

(event `/Game/Blueprints/BPI_Item.UsePrimary`
  ; Spawns a little guy
  (`KismetSystemLibrary.PrintText` "Activating primary action")
  (`|SpawnActorFromClass` "/Game/AI_Blueprints/BP_AiMoveTo.BP_AiMoveTo_C" (`self.GetTransform`) "Undefined" "MultiplyWithRoot" null null))

(event `/Game/Blueprints/BPI_Item.UseSecondary`
  ; Changes material of wand to an emissive
  (`KismetSystemLibrary.PrintText` "Activating secondary action")
  (`/Engine/EditorBlueprintResources/StandardMacros.FlipFlop`
    (:`A`
      (`PrimitiveComponent.SetMaterial` (`self.Cylinder`) 0 "/Game/Materials/MI_EmissivePink.MI_EmissivePink"))
    (:`B`
      (`PrimitiveComponent.SetMaterial` (`self.Cylinder`) 0 "/Game/Materials/M_Base.M_Base"))))

(event `/Game/Blueprints/BPI_Item.Drop`
  ; Drops wand
  (`KismetSystemLibrary.PrintText` "Dropping item")
  (`self.K2_DetachFromActor` "KeepWorld")
  (`|SpawnActorFromClass` "BP_SummoningWand_C" (`self.GetTransform`) "Undefined" "MultiplyWithRoot" null null)
  (`self.K2_DestroyActor`))

(fn `UserConstructionScript`)