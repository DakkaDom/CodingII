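; BP_PatrolRoute is an actor that defines an AI patrol route with a spline and supplies patrol point locations.
; Each GetPatrolPointLocation call steps PatrolIndex by Direction and returns that spline point in world space.
; Direction reverses at either end for back-and-forth movement.
; The end check follows the increment, so the index can equal the point count during lookup.
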(fn `GetPatrolPointLocation`
  (returns (Location :type "Vector Structure"))
  (set `self.PatrolIndex` (+ (`self.PatrolIndex`) (`self.Direction`))) ; Go to "next" point
  (if (>= (`self.PatrolIndex`) (`SplineComponent.GetNumberOfSplinePoints` (`self.Spline`)))
    (set `self.Direction` -1) ; Reverse the direction
    (elif (<= (`self.PatrolIndex`) 0)
      (set `self.Direction` 1) ; Reverse the direction
    ))
  (return (`SplineComponent.GetLocationAtSplinePoint` (`self.Spline`) (`self.PatrolIndex`) "World")))

(fn `UserConstructionScript`)